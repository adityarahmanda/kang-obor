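; KangOborController is a player controller that handles shooting and mouse aiming for its possessed character.
; Fire press turns off orient-rotation-to-movement, flags shooting and sets the controller's rotation from a cursor trace, feeding look-at pitch into roll; release restores movement orientation.
; While Fire is held, a Tick gate calls an empty SetAimAngle and yaws the pawn through FlipPlayer whenever LookAngle exceeds ninety degrees either side.
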(event Custom|Stop%20Fire
  ;[1 1 1] Start and Stop Fire
  (Variables|/Script/Engine.CharacterMovementComponent|SetbOrientRotationToMovement (Variables|/Script/Engine.Character|GetCharacterMovement (.CharacterReference (Variables|Default|GetCharacterReference))) true)
  (Variables|Default|SetIsShooting false))

(event Custom|Start%20Fire
  ;[1 1 1] Start and Stop Fire
  (Variables|/Script/Engine.CharacterMovementComponent|SetbOrientRotationToMovement (Variables|/Script/Engine.Character|GetCharacterMovement (.CharacterReference (Variables|Default|GetCharacterReference))) false)
  (Variables|Default|SetIsShooting true)
  (CallFunction|RotatetoAim))

(event EventTick
  (params (DeltaSeconds :type Float%20%28single-precision%29))
  (bind _lookangle (Variables|Default|GetLookAngle))
  ;[1 1 1] InputAction Fire
  (Utilities|FlowControl|Gate true
    (:Exit
      (CallFunction|SetAimAngle)
      (if (or (> _lookangle 9e+01) (< _lookangle -9e+01))
        (CallFunction|FlipPlayer)))))

(event EventBeginPlay
  ;[1 1 1] BeginPlay
  (bind _astop_down_character (Utilities|Casting|CastTo (Pawn|GetControlledPawn)))
  (Variables|Default|SetCharacterReference 0 _astop_down_character))

(event Input|ActionEvents|InputActionFire
  (params (Key :type Key%20Structure))
  (bind _lookangle (Variables|Default|GetLookAngle))
  ;[1 1 1] InputAction Fire
  (:Pressed
    (CallFunction|StartFire)
    (Utilities|FlowControl|Gate true) ; enters at Open
  )
  (:Released
    (CallFunction|StopFire)
    (Utilities|FlowControl|Gate true) ; enters at Close
  ))

(fn ConstructionScript)

(fn RotatetoAim
  (Transformation|SetActorRotation (Math|Rotator|MakeRotator (.Pitch (Math|Rotator|BreakRotator (Math|Rotator|FindLookatRotation (Transformation|GetActorLocation (Pawn|GetControlledPawn)) (.Location (Collision|BreakHitResult (.HitResult (Game|Player|GetHitResultUnderCursorbyChannel "TraceTypeQuery1" true))))))) 0.0 0.0)))

(fn SetAimAngle)

(fn FlipPlayer
  (bind _returnvalue (Pawn|GetControlledPawn))
  (bind _returnvalue_2 (Transformation|GetActorRotation _returnvalue))
  (bind (_roll _pitch _yaw) (Math|Rotator|BreakRotator _returnvalue_2))
  (Transformation|SetActorRotation _returnvalue (Math|Rotator|MakeRotator _roll _pitch (+ _yaw 1e+02))))