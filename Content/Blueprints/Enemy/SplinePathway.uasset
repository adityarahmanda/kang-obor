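; Spline pathway actor in the Enemy folder that moves a reference point along a spline at a set speed.
; Each Tick it advances a travelled distance by Speed and delta time, then places ReferencePoint at that world-space spline location without sweeping.
; When IsLooping is set, the distance resets to zero past the spline's end; otherwise it keeps accumulating.
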(event EventTick
  (params (DeltaSeconds :type Float%20%28single-precision%29))
  (Variables|Default|SetDistance (+ (* DeltaSeconds (Variables|Default|GetSpeed)) (Variables|Default|GetDistance)))
  (bind _output_get (Variables|Default|SetLocation (Spline|GetLocationatDistanceAlongSpline (Variables|Default|GetSpline) (Variables|Default|GetDistance) "World")))
  (Transformation|SetWorldLocation (Variables|Default|GetReference%20Point) _output_get false false)
  (if (Variables|Default|GetIsLooping)
    (if (> (Variables|Default|GetDistance) (Spline|GetSplineLength (Variables|Default|GetSpline)))
      (Variables|Default|SetDistance 0.0))))

(fn ConstructionScript)