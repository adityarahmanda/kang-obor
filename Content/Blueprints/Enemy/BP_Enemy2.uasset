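; BP_Enemy2 is an enemy Blueprint that damages the player through an attack collision overlap.
; When a player character enters AttackCollision, it calls the player's TakeDamage with its Damage value and itself as the hit actor, but only while the enemy is attacking and the player is not already hit.
; The construction script only calls the parent, and this file does not set the attack state.
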(event OnComponentBeginOverlap(AttackCollision)
  (params (OverlappedComponent :type Primitive%20Component%20Object%20Reference) (OtherActor :type Actor%20Object%20Reference) (OtherComp :type Primitive%20Component%20Object%20Reference) (OtherBodyIndex :type Integer) (bFromSweep :type Boolean) (SweepResult :type Hit%20Result%20Structure%20%28by%20ref%29))
  (bind _asbp_player_character (Utilities|Casting|CastToBP_PlayerCharacter OtherActor))
  (if (and (not (Variables|/Game/Blueprints/Player/BP_PlayerCharacter.BP_PlayerCharacter_C|GetisHit _asbp_player_character)) (Variables|Default|GetIsAttacking))
    (Default|TakeDamage _asbp_player_character (Variables|Default|GetDamage) self)))

(fn ConstructionScript
  (|CallParentFunction))