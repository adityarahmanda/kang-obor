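; Behavior tree task that sends an enemy to a location stored in the blackboard while the player is in range.
; On execute, it casts the owner to Enemy_AI and starts a move to the target location.
; Each tick it writes the player range check to the blackboard, finishing successfully when movement goes idle, or stopping movement and also finishing successfully if the player is out of range.
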(event EventReceiveExecuteAI
  (params (OwnerController :type AI%20Controller%20Object%20Reference) (ControlledPawn :type Pawn%20Object%20Reference))
  (bind _asenemy_ai (Utilities|Casting|CastToEnemy_AI OwnerController))
  (bind _output_get (Variables|Default|SetControllerRef _asenemy_ai))
  (AI|Navigation|MovetoLocation _output_get (Class|BTFunctionLibrary|GetBlackboardValueasVector (Variables|Default|GetTargetLocation_Ref)) 0.0 true true false true 0))

(event EventReceiveTickAI
  (params (OwnerController :type AI%20Controller%20Object%20Reference) (ControlledPawn :type Pawn%20Object%20Reference) (DeltaSeconds :type Float%20%28single-precision%29))
  (bind _inrangeplayer (Default|InRangePlayer (Variables|Default|GetControllerRef) (Variables|Default|GetInPlayerRangeDistance)))
  (Class|BTFunctionLibrary|SetBlackboardValueasBool (Variables|Default|GetInRangePlayer_Ref) _inrangeplayer)
  (if _inrangeplayer
    (if (Utilities|Enum|Equal(Enum) (Class|AIController|GetMoveStatus (Variables|Default|GetControllerRef)) "Idle")
      (AI|BehaviorTree|FinishExecute true))
    (else
      (AI|Navigation|StopMovement (Variables|Default|GetControllerRef))
      (AI|BehaviorTree|FinishExecute true))))