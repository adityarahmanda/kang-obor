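; Enemy AI controller that runs the Enemy_BT behavior tree for a controlled BP_EnemyBase pawn.
; AI perception updates write whether the player character is sensed to the CanSeePlayer blackboard key.
; Helper functions check range to the player and compute attack points on the player-to-enemy line, plus strafe points offset randomly to the enemy's left or right.
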(event OnTargetPerceptionUpdated(AIPerception)
  (params (Actor :type Actor%20Object%20Reference) (Stimulus :type AI%20Stimulus%20Structure))
  (bind _bsuccessfullysensed (Utilities|Struct|BreakAIStimulus Stimulus))
  (Utilities|Casting|CastToBP_PlayerCharacter Actor)
  (AI|Components|Blackboard|SetValueasBool (AI|GetBlackboard 0) (Utilities|Name|MakeLiteralName "CanSeePlayer") _bsuccessfullysensed)
  (if _bsuccessfullysensed
    _))

(event EventBeginPlay
  (bind _asbp_enemy_base (Utilities|Casting|CastToBP_EnemyBase (Pawn|GetControlledPawn)))
  (Variables|Default|SetEnemyReference _asbp_enemy_base)
  (AI|RunBehaviorTree "/Game/Blueprints/Enemy/Enemy_BT.Enemy_BT"))

(fn ConstructionScript)

(fn GetStrafingPosition
  (params (StrafeDistance :type Float%20%28single-precision%29) (DistanceFromPlayer :type Float%20%28single-precision%29))
  (bind _returnvalue (Game|Player|GetPlayerPawn 0))
  (bind _returnvalue_2 (Game|Player|GetPlayerPawn 0))
  (bind _enemyreference (Variables|Default|GetEnemyReference))
  (bind _enemyreference_2 (Variables|Default|GetEnemyReference))
  (bind _returnvalue_3 (Transformation|GetActorLocation _returnvalue))
  (bind _returnvalue_4 (Transformation|GetActorLocation _returnvalue_2))
  (if (Math|Random|RandomBool)
    (return (+ _returnvalue_3 (* (Math|Vector|GetForwardVector (Math|Rotator|FindLookatRotation _returnvalue_3 (Transformation|GetActorLocation _enemyreference))) DistanceFromPlayer) (* (Transformation|GetActorRightVector _enemyreference) StrafeDistance)))
    (else
      (return (+ _returnvalue_4 (* (Math|Vector|GetForwardVector (Math|Rotator|FindLookatRotation _returnvalue_4 (Transformation|GetActorLocation _enemyreference_2))) DistanceFromPlayer) (* (Transformation|GetActorRightVector _enemyreference_2) (* StrafeDistance -1.0)))))))

(fn InRangePlayer
  (params (Range :type Float%20%28single-precision%29))
  (return (<= (Transformation|GetDistanceTo (Variables|Default|GetEnemyReference) (Game|Player|GetPlayerPawn 0)) Range)))

(fn GetAttackLocation
  (params (DistanceFromPlayer :type Float%20%28single-precision%29))
  (bind _returnvalue (Game|Player|GetPlayerPawn 0))
  (bind _returnvalue_2 (Transformation|GetActorLocation _returnvalue))
  (return (+ _returnvalue_2 (* (Math|Vector|GetForwardVector (Math|Rotator|FindLookatRotation _returnvalue_2 (Transformation|GetActorLocation (Variables|Default|GetEnemyReference)))) DistanceFromPlayer))))