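; BP_EnemyBase is a base enemy Blueprint that manages walk speed and attack and hit states.
; BeginPlay caches the initial max walk speed, then matches movement speed to the SplinePath speed, with a function to restore normal speed.
; Attack only starts when neither attacking nor hit, and taking damage cancels an attack and flags the hit.
; CheckInRangePlayer is an empty stub, and neither flag is reset here.
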(event Custom|Attack
  ;[1 1 1] Event Attack
  (if (not (Variables|Default|GetIsAttacking))
    (if (not (Variables|Default|GetIsHit))
      (Variables|Default|SetIsAttacking true))))

(event EventBeginPlay
  ;[1 1 1] Begin Play
  (Variables|Default|SetInitMaxWalkSpeed (Variables|/Script/Engine.CharacterMovementComponent|GetMaxWalkSpeed (Variables|Character|GetCharacterMovement)))
  (CallFunction|SetWalkMovementSpeedtoSplineSpeed))

(event EventTakeDamage
  (params (Damage :type Float%20%28single-precision%29) (Hit%20Actor :type Actor%20Object%20Reference))
  ;[1 1 1] Event Take Damage
  (if (not (Variables|Default|GetIsHit))
    (Variables|Default|SetIsAttacking false)
    (Variables|Default|SetIsHit true)))

(fn ConstructionScript)

(fn SetWalkMovementSpeedtoSplineSpeed
  (Variables|/Script/Engine.CharacterMovementComponent|SetMaxWalkSpeed (Variables|Character|GetCharacterMovement) (Variables|/Game/Blueprints/Enemy/SplinePathway.SplinePathway_C|GetSpeed (Variables|Default|GetSplinePath))))

(fn SetWalkMovementSpeedtoNormal
  (Variables|/Script/Engine.CharacterMovementComponent|SetMaxWalkSpeed (Variables|Character|GetCharacterMovement) (Variables|Default|GetInitMaxWalkSpeed)))

(fn CheckinRangePlayer)