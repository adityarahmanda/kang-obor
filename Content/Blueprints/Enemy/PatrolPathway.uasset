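; PatrolPathway is an enemy patrol Blueprint that moves a referenced actor along its spline.
; Each tick it advances a distance by Speed scaled by delta time, then sets the actor's world location to that point without sweeping or changing rotation.
; When IsLooping is set, passing the spline's end resets the distance to zero, so the actor restarts from the beginning.
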(event EventTick
  (params (DeltaSeconds :type Float%20%28single-precision%29))
  (Variables|Default|SetDistance (+ (* DeltaSeconds (Variables|Default|GetSpeed)) (Variables|Default|GetDistance)))
  (Transformation|SetActorLocation (Variables|Default|GetPatrolActorRef) (Spline|GetLocationatDistanceAlongSpline (Variables|Default|GetSpline) (Variables|Default|GetDistance) "World") false false)
  (if (Variables|Default|GetIsLooping)
    (if (> (Variables|Default|GetDistance) (Spline|GetSplineLength (Variables|Default|GetSpline)))
      (Variables|Default|SetDistance 0.0))))

(fn ConstructionScript)